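; BP_JeonPlayer is a player actor that moves on the Y-Z plane from Enhanced Input.
; BeginPlay adds the IMC_Default mapping context to the first player controller's input subsystem.
; IA_Move maps its 2D value to Y and Z, normalizes it, scales it by Jspeed and delta time, and offsets the actor location without sweep, so movement does not stop on collisions.
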(event `self.ReceiveBeginPlay`
  ;[1 1 1] Player가 시작하면 Keyboard Input 입력을 설정하겠다
  ;;[1 1 1] 처음 시작하면
  ;;[1 1 1] Keyboard input을 설정한다
  (`EnhancedInputSubsystemInterface.AddMappingContext` (pcsubsystem `EnhancedInputLocalPlayerSubsystem` (`GameplayStatics.GetPlayerController` 0)) "/Game/ThirdPerson/Input/IMC_Default.IMC_Default" 0 (struct)))

(event `EnhancedInput|/Game/ThirdPerson/Input/Actions/IA_Move`
  (params (ActionValue :type "Vector2D Structure") (ElapsedSeconds :type "Float (double-precision)") (TriggeredSeconds :type "Float (double-precision)") (InputAction :type "InputAction Object Reference" :default "/Game/ThirdPerson/Input/Actions/IA_Move.IA_Move"))
  ;[1 1 1] Charactor에 Input이 들어오면 그 방향대로 위치를 설정하고 싶다.
  (:`Triggered`
    (`self.K2_SetActorLocation` (+ (* (`KismetMathLibrary.Normal` (`KismetMathLibrary.MakeVector` 0.0 ActionValue_X ActionValue_Y)) (* (`GameplayStatics.GetWorldDeltaSeconds`) (`self.jspeed`))) (`self.K2_GetActorLocation`)))))

(fn `UserConstructionScript`)